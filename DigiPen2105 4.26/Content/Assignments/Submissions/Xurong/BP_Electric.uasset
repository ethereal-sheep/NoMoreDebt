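; BP_Electric is a hazard actor that deals damage over time to actors inside its damage volume, a component named Goo.
; Overlap begin and end maintain a unique array of damageable actors, starting the DamageOverTime timeline when it has entries and stopping it when empty.
; Each timeline update applies DamagePerTick to every listed actor, so damage lands per update rather than being scaled by elapsed time.
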(event OnComponentBeginOverlap(Goo)
  (params (OverlappedComponent :type Primitive%20Component%20Object%20Reference) (OtherActor :type Actor%20Object%20Reference) (OtherComp :type Primitive%20Component%20Object%20Reference) (OtherBodyIndex :type Integer) (bFromSweep :type Boolean) (SweepResult :type Hit%20Result%20Structure%20%28by%20ref%29))
  ;[1 1 1] Detect Actors entering / leaving Damage Volume
  (if (Variables|/Script/Engine.Actor|GetbCanBeDamaged OtherActor)
    (Utilities|Array|AddUnique (Variables|Default|GetArray_of_Actors_To_Damage) OtherActor)
    ;[1 1 1] Only activate Timeline IF there are actors in the damage volume
    (if (> (Utilities|Array|Length (Variables|Default|GetArray_of_Actors_To_Damage)) 0)
      (CallFunction|STARTDAMAGE)
      (else
        (CallFunction|STOPDAMAGE)))))

(event OnComponentEndOverlap(Goo)
  (params (OverlappedComponent :type Primitive%20Component%20Object%20Reference) (OtherActor :type Actor%20Object%20Reference) (OtherComp :type Primitive%20Component%20Object%20Reference) (OtherBodyIndex :type Integer))
  ;[1 1 1] Detect Actors entering / leaving Damage Volume
  (if (Utilities|Array|ContainsItem (Variables|Default|GetArray_of_Actors_To_Damage) OtherActor)
    (Utilities|Array|RemoveItem (Variables|Default|GetArray_of_Actors_To_Damage) OtherActor)
    ;[1 1 1] Only activate Timeline IF there are actors in the damage volume
    (if (> (Utilities|Array|Length (Variables|Default|GetArray_of_Actors_To_Damage)) 0)
      (CallFunction|STARTDAMAGE)
      (else
        (CallFunction|STOPDAMAGE)))))

(event Custom|START_DAMAGE
  ;[1 1 1] Cause Damage to Actors in Damage Volume
  (if (not (Audio|Components|Audio|IsPlaying (Variables|Default|GetDamage_Over_Time)))
    (Timeline|Damage_Over_Time Play
      (:Update
        (for _array_element (Variables|Default|GetArray_of_Actors_To_Damage)
          (Game|Damage|ApplyDamage _array_element (Variables|Default|GetDamage_per_Tick) 0 0))))))

(event Custom|STOP_DAMAGE
  ;[1 1 1] Cause Damage to Actors in Damage Volume
  (if (Audio|Components|Audio|IsPlaying (Variables|Default|GetDamage_Over_Time))
    (Timeline|Damage_Over_Time Stop
      (:Update
        (for _array_element (Variables|Default|GetArray_of_Actors_To_Damage)
          (Game|Damage|ApplyDamage _array_element (Variables|Default|GetDamage_per_Tick) 0 0))))))

(fn ConstructionScript)