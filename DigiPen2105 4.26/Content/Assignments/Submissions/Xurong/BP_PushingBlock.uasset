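; BP_PushingBlock is a hazard block that repeatedly extends and retracts, launching characters that overlap its Box.
; A timeline stretches the Arrow component along X after a start delay and reverses after a return delay.
; Tick checks whether the Arrow is fully extended to choose between push and return, calling one of them every frame.
; Box overlap launches the character by Pushvector, overriding its existing velocity.
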(event OnComponentBeginOverlap(Box)
  (params (OverlappedComponent :type Primitive%20Component%20Object%20Reference) (OtherActor :type Actor%20Object%20Reference) (OtherComp :type Primitive%20Component%20Object%20Reference) (OtherBodyIndex :type Integer) (bFromSweep :type Boolean) (SweepResult :type Hit%20Result%20Structure%20%28by%20ref%29))
  (bind _ascharacter (Utilities|Casting|CastToCharacter OtherActor))
  (Character|LaunchCharacter _ascharacter (Variables|Default|GetPushvector) true true))

(event Custom|Return
  (Utilities|FlowControl|Delay (Variables|Default|GetReturnDelay))
  (bind _1_3 (Timeline|Timeline_0 Reverse)
    (:Update
      (Transformation|SetRelativeScale3D (Variables|Default|GetArrow) (Math|Vector|Lerp(Vector) "1.000000,1.000000,1.000000" "4.000000,1.000000,1.000000" _1_3)))))

(event Custom|Push
  (Utilities|FlowControl|Delay (Variables|Default|GetStartDelay))
  (bind _1_3 (Timeline|Timeline_0 Play)
    (:Update
      (Transformation|SetRelativeScale3D (Variables|Default|GetArrow) (Math|Vector|Lerp(Vector) "1.000000,1.000000,1.000000" "4.000000,1.000000,1.000000" _1_3)))))

(event Collision|EventActorBeginOverlap
  (params (OtherActor :type Actor%20Object%20Reference)))

(event EventTick
  (params (DeltaSeconds :type Float%20%28single-precision%29))
  (if (Math|Vector|Equal(Vector) (Variables|/Script/Engine.SceneComponent|GetRelativeScale3D (Variables|Default|GetArrow)) "4.000000,1.000000,1.000000" 0.0001)
    (Variables|Default|SetEnded true)
    (else
      (Variables|Default|SetEnded false)))
  (if (Variables|Default|GetEnded)
    (CallFunction|Return)
    (else
      (CallFunction|Push))))

(fn ConstructionScript)